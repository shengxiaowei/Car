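; Test vehicle actor that follows a BPSpline path, started and stopped with Ctrl+S and Ctrl+P.
; Each tick advances spline distance, then derives a smoothed ground-conforming transform from downward traces at four yaw-rotated corner offsets.
; Steering yaw comes from the signed angle to a look-ahead spline tangent, with debug prints and drawing.
; Curve-based speed reduction in GetTargetSpeed is unconnected, as is the wheel-spin timeline update.
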(event `Key|Ctrl+S`
  (params (Key :type "Key Structure"))
  ;[1 1 1] 开始运动
  (:`Pressed`
    (`self.StartRun`)))

(event `Key|Ctrl+P`
  (params (Key :type "Key Structure"))
  ;[1 1 1] 停止运动
  (:`Pressed`
    (`self.StopRun`)))

(event `self.ReceiveTick`
  (params (DeltaSeconds :type "Float (single-precision)"))
  (if (`self.IsRun`)
    (bind _transform (`self.CalcTransform` DeltaSeconds))
    (`self.K2_SetActorTransform` _transform)
    (`TimelineComponent.SetPlayRate` (`self.TL_wheelRotate`) (/ (`self.CurrentCarSpeed`) 2.0))))

(fn `Calc Wheel`
  (params (Location :type "Vector Structure") (Rotation :type "Rotator Structure"))
  (returns (NewTransform :type "Transform Structure"))
  (bind _yaw (.yaw Rotation))
  (bind _newlocation (`self.GetLocation` (+ Location (`KismetMathLibrary.RotateAngleAxis` (`self.LF`) _yaw (0.0 0.0 1.0)))))
  (bind _newlocation_2 (`self.GetLocation` (+ Location (`KismetMathLibrary.RotateAngleAxis` (`self.RB`) _yaw (0.0 0.0 1.0)))))
  (bind _newlocation_3 (`self.GetLocation` (+ Location (`KismetMathLibrary.RotateAngleAxis` (`self.LB`) _yaw (0.0 0.0 1.0)))))
  (bind _newlocation_4 (`self.GetLocation` (+ Location (`KismetMathLibrary.RotateAngleAxis` (`self.RF`) _yaw (0.0 0.0 1.0)))))
  (bind _returnvalue (`KismetMathLibrary.MakeRotFromXY` (- (/ (+ _newlocation_4 _newlocation) 2.0) (/ (+ _newlocation_2 _newlocation_3) 2.0)) (- (/ (+ _newlocation_4 _newlocation_2) 2.0) (/ (+ _newlocation _newlocation_3) 2.0))))
  (`KismetSystemLibrary.PrintString` (`KismetStringLibrary.Conv_DoubleToString` _yaw) true true (struct :`G` 0.66 :`B` 1.0 :`A` 1.0) 0.0)
  (set `self.NewVar_0` (`KismetMathLibrary.RInterpTo` (`self.NewVar_0`) _returnvalue (`GameplayStatics.GetWorldDeltaSeconds`) 2.0))
  (bind _output_get (set `self.NewVar_2` (`KismetMathLibrary.TInterpTo` (`self.NewVar_2`) (`KismetMathLibrary.MakeTransform` (`KismetMathLibrary.GetVectorArrayAverage` (`|MakeArray` _newlocation_4 _newlocation _newlocation_2 _newlocation_3)) _returnvalue) (`GameplayStatics.GetWorldDeltaSeconds`) 5.0)))
  (return _output_get))

(fn `CalcTransform`
  (params (Time :type "Float (double-precision)"))
  (returns (Transform :type "Transform Structure"))
  (bind _bp_spline (`self.BP_Spline`))
  (if (< (`self.CurrentLength`) (`self.Length`))
    (bind _output_get (set `self.TargetSpeed` (`self.GetTargetSpeed`)))
    (`/Engine/EditorBlueprintResources/StandardMacros.IsValid` _bp_spline
      (:`Is Valid`
        (bind _returnvalue (+ (* Time _output_get) (`self.CurrentLength`)))
        (set `self.CurrentLength` _returnvalue)
        (bind _transform (`/Game/BPVehicle/BP_Line.GetTransformByLen` _bp_spline _returnvalue))
        (bind _newtransform (`self.Calc Wheel` (.location _transform) (.rotation _transform)))
        (`self.CalcWheelSteer` _returnvalue)
        (bind _returnvalue_2 (`PrimitiveComponent.GetPhysicsLinearVelocity` (`self.chesheng`) "None"))
        (bind _output_get_2 (set `self.CurrentCarSpeed` (/ (+ (`KismetMathLibrary.VSize` _returnvalue_2) 11.0) 100.0)))
        (`KismetSystemLibrary.PrintString` (`KismetStringLibrary.Concat_StrStr` "车速：" (`KismetStringLibrary.Conv_DoubleToString` _output_get_2)) true false (struct :`G` 0.66 :`B` 1.0 :`A` 1.0) (`GameplayStatics.GetWorldDeltaSeconds`))
        (return _newtransform)))))

(fn `CalcWheelSteer`
  (params (InputPin :type "Float (double-precision)"))
  (bind _returnvalue (+ InputPin 400.0))
  (bind _spline (`/Game/BPVehicle/BP_Line.Spline` (`self.BP_Spline`)))
  (bind _returnvalue_2 (`SplineComponent.GetDirectionAtDistanceAlongSpline` _spline InputPin "World"))
  (bind _returnvalue_3 (`SplineComponent.GetTangentAtDistanceAlongSpline` _spline _returnvalue "World"))
  (bind _returnvalue_4 (* (`KismetMathLibrary.DegAcos` (`KismetMathLibrary.DotProduct2D` (`KismetMathLibrary.Normal2D` (`KismetMathLibrary.Conv_VectorToVector2D` _returnvalue_2)) (`KismetMathLibrary.Normal2D` (`KismetMathLibrary.Conv_VectorToVector2D` _returnvalue_3)))) (`KismetMathLibrary.SelectFloat` 1.0 -1.0 (> (.z (`KismetMathLibrary.Cross_VectorVector` _returnvalue_2 _returnvalue_3)) 0.0))))
  (bind _output_get (set `self.Car_Yaw` (`KismetMathLibrary.FInterpTo` (`self.Car_Yaw`) (* _returnvalue_4 (`self.steerStrength`)) (`GameplayStatics.GetWorldDeltaSeconds`) 5.0)))
  (`KismetSystemLibrary.PrintString` (`KismetStringLibrary.Concat_StrStr` "车身航道偏差角度：" (`KismetStringLibrary.Conv_DoubleToString` (`KismetMathLibrary.Abs` _returnvalue_4))) true false (struct :`R` 1.0 :`B` 0.037586 :`A` 1.0) (`GameplayStatics.GetWorldDeltaSeconds`))
  (`SceneComponent.K2_SetRelativeRotation` (`self.Box`) (`KismetMathLibrary.MakeRotator` 0.0 0.0 _output_get) false false)
  (`SceneComponent.K2_SetRelativeRotation` (`self.Box2`) (`KismetMathLibrary.MakeRotator` 0.0 0.0 _output_get) false false)
  (`KismetSystemLibrary.DrawDebugPoint` (`SplineComponent.GetLocationAtDistanceAlongSpline` _spline _returnvalue "World") 11.0 (struct :`R` 1.0 :`G` 0.017706 :`B` 0.147432 :`A` 1.0) 1.0))

(fn `GetLocation`
  (params (Start :type "Vector Structure"))
  (returns (NewLocation :type "Vector Structure"))
  (bind _x (.x Start))
  (bind _y (.y Start))
  (bind _z (.z Start))
  (bind _outhit (`KismetSystemLibrary.LineTraceSingle` :`Start` (`KismetMathLibrary.MakeVector` _x _y (+ _z 1000.0)) :`End` (`KismetMathLibrary.MakeVector` _x _y (- _z 1000.0)) :`TraceChannel` "TraceTypeQuery1" :`DrawDebugType` "ForOneFrame"))
  (return (`.Location` (`GameplayStatics.BreakHitResult` _outhit))))

(fn `StartRun`
  (bind _bp_spline (`self.BP_Spline`))
  (set `self.CurrentLength` 0.0)
  (`/Engine/EditorBlueprintResources/StandardMacros.IsValid` _bp_spline
    (:`Is Valid`
      (bind _linelength (`/Game/BPVehicle/BP_Line.GetLength` _bp_spline))
      (set `self.Length` _linelength)
      (set `self.IsRun` true))))

(fn `StopRun`
  (set `self.IsRun` false))

(fn `UserConstructionScript`)